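; Samurai character for a quick-draw duel, drawn as a Paper2D sprite that slides into place on BeginPlay.
; Its Attack event allows one press, checked against the GM_Duel phase: pressing during Wait shows a cross and uses up the press.
; Pressing during Draw plays a timeline that lerps the sprite to the attack position and swaps in the Tanuki attack sprite.
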(event Custom|SlideIn
  (Components|Timeline|SetPlayRate (Variables|Default|GetSlideInAnim) 2.0)
  (bind _alpha (Timeline|SlideInAnim PlayFromStart)
    (:Update
      (Transformation|SetRelativeLocation (Variables|Default|GetPaperSprite) (Math|Vector|Lerp(Vector) (Variables|Default|GetSlide%20Start%20Pos) (Variables|Default|GetSprit%20Default%20Pos) _alpha) false false))))

(event Custom|Attack
  (if (not (Variables|Default|GetPressedDraw))
    (switch Utilities|FlowControl|Switch|SwitchonE_Phase (Variables|/Game/Dynamic/Blueprints/GM_Duel.GM_Duel_C|GetPhase (Variables|Default|GetGameMode))
      (:NewEnumerator1
        (CallFunction|SetCrossVisibility true)
        (Variables|Default|SetPressedDraw true))
      (:NewEnumerator2
        (Variables|Default|SetPressedDraw true)
        (Components|Timeline|SetPlayRate (Variables|Default|GetAttackAnim) 8.0)
        (bind _alpha (Timeline|AttackAnim PlayFromStart)
          (:Update
            (Transformation|SetRelativeLocationAndRotation (Variables|Default|GetPaperSprite) (Math|Vector|Lerp(Vector) (Variables|Default|GetSprit%20Default%20Pos) (Variables|/Script/Engine.SceneComponent|GetRelativeLocation (Variables|Default|GetAttackPos)) _alpha) "0, 0, 0" false false))
          (:SwitchSprite
            (CallFunction|SetSprit "/Game/Static/Tanuki/T_Tanuki_Attack_Sprite.T_Tanuki_Attack_Sprite")))))))

(event EventBeginPlay
  (bind _asgm_duel (Utilities|Casting|CastToGM_Duel (Game|GetGameMode)))
  (Variables|Default|SetGameMode _asgm_duel)
  (Variables|Default|SetSprit%20Default%20Pos (Variables|/Script/Engine.SceneComponent|GetRelativeLocation (Variables|Default|GetPaperSprite)))
  (CallFunction|Slidein)
  (CallFunction|SetCrossVisibility false))

(fn ConstructionScript)

(fn SetCrossVisibility
  (params (bNewVisibility :type Boolean))
  (Rendering|SetVisibility (Variables|Default|GetCross) bNewVisibility false))

(fn SetSprit
  (params (NewSprite :type Paper%20Sprite%20Object%20Reference))
  (Rendering|Components|Sprite|SetSprite (Variables|Default|GetPaperSprite) NewSprite)
  (Rendering|Material|SetMaterial (Variables|Default|GetPaperSprite) 0 "/Paper2D/TranslucentUnlitSpriteMaterial.TranslucentUnlitSpriteMaterial")
  (Rendering|SetTranslucentSortPriority (Variables|Default|GetPaperSprite) 1))